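; BP_Spawner is an actor that drops balls at random points inside its Box component in two timed waves.
; From BeginPlay, a looping timer spawns BP_InteractableBall until a delay in its event pauses it.
; That same event then starts a second looping timer spawning BP_Ball, which is paused after another delay.
; Intervals and stop delays come from separate variables for each wave.
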(event `self.ReceiveBeginPlay`
  (bind _returnvalue (`KismetSystemLibrary.K2_SetTimerDelegate` (delegate `SpawnInteract`) (`self.Time_0`) true))
  (set `self.Set chrono_01` _returnvalue))

(event `SpawnInteract`
  (bind _box (`self.Box`))
  (`|SpawnActorFromClass` "/Game/Game/TopDownShooter/Maps/InteractableObject/Boules/BP_InteractableBall.BP_InteractableBall_C" (`KismetMathLibrary.MakeTransform` (`KismetMathLibrary.RandomPointInBoundingBox` (`SceneComponent.K2_GetComponentLocation` _box) (`BoxComponent.BoxExtent` _box))) "Undefined" "MultiplyWithRoot" null null)
  (`KismetSystemLibrary.Delay` (`self.Temps_darret_0`))
  (`KismetSystemLibrary.K2_PauseTimerHandle` (`self.Set chrono_01`))
  (bind _returnvalue (`KismetSystemLibrary.K2_SetTimerDelegate` (delegate `Spawn`) (`self.Time`) true))
  (set `self.Set chrono` _returnvalue)
  (`KismetSystemLibrary.Delay` (`self.Temps_darret`))
  (`KismetSystemLibrary.K2_PauseTimerHandle` (`self.Set chrono`)))

(event `Spawn`
  (bind _box (`self.Box`))
  (`|SpawnActorFromClass` "/Game/Game/TopDownShooter/Maps/InteractableObject/Boules/BP_Ball.BP_Ball_C" (`KismetMathLibrary.MakeTransform` (`KismetMathLibrary.RandomPointInBoundingBox` (`SceneComponent.K2_GetComponentLocation` _box) (`BoxComponent.BoxExtent` _box))) "Undefined" "MultiplyWithRoot" null null))

(fn `UserConstructionScript`)